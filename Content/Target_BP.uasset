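; Target actor that pitches up to standing or back down as the first-person player character enters or leaves either of two referenced trigger actors, Trr1 and Trr2.
; Begin overlap calls stand and end overlap calls Down, each playing its own timeline to rotate the root's pitch.
; Currentstatus gates both moves through Up, Ready and Down, so calls arriving mid-rotation are ignored rather than queued.
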(event OnActorBeginOverlap(trr1)
  (params (OverlappedActor :type Actor%20Object%20Reference) (OtherActor :type Actor%20Object%20Reference))
  (Utilities|Casting|CastToBP_FirstPersonCharacter_Child OtherActor)
  (CallFunction|Stand))

(event OnActorBeginOverlap(trr2)
  (params (OverlappedActor :type Actor%20Object%20Reference) (OtherActor :type Actor%20Object%20Reference))
  (Utilities|Casting|CastToBP_FirstPersonCharacter_Child OtherActor)
  (CallFunction|Stand))

(event OnActorEndOverlap(trr1)
  (params (OverlappedActor :type Actor%20Object%20Reference) (OtherActor :type Actor%20Object%20Reference))
  (Utilities|Casting|CastToBP_FirstPersonCharacter_Child OtherActor)
  (CallFunction|Down))

(event OnActorEndOverlap(trr2)
  (params (OverlappedActor :type Actor%20Object%20Reference) (OtherActor :type Actor%20Object%20Reference))
  (Utilities|Casting|CastToBP_FirstPersonCharacter_Child OtherActor)
  (CallFunction|Down))

(event Custom|Down
  (switch Utilities|FlowControl|Switch|Switchontarget_state (Variables|Default|GetCurrentstatus)
    (:NewEnumerator1
      (Variables|Default|SetCurrentstatus "NewEnumerator0")
      (bind _새_트랙_0 (Timeline|타임라인_0 PlayFromStart)
        (:Update
          (Transformation|SetRelativeRotation (Variables|Default|GetDefaultSceneRoot) (Math|Rotator|MakeRotator 0.0 _새_트랙_0 0.0) false false))
        (:Finished
          (Variables|Default|SetCurrentstatus "NewEnumerator2"))))))

(event Custom|stand
  (switch Utilities|FlowControl|Switch|Switchontarget_state (Variables|Default|GetCurrentstatus)
    (:NewEnumerator2
      (Variables|Default|SetCurrentstatus "NewEnumerator0")
      (bind _새_트랙_0 (Timeline|타임라인 PlayFromStart)
        (:Update
          (Transformation|SetRelativeRotation (Variables|Default|GetDefaultSceneRoot) (Math|Rotator|MakeRotator 0.0 _새_트랙_0 0.0) false false))
        (:Finished
          (Variables|Default|SetCurrentstatus "NewEnumerator1"))))))

(fn ConstructionScript)