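; Bullet projectile actor that knocks down Target_BP actors it hits and then destroys itself.
; Each tick it moves along its forward vector at Speed, scaled by delta time, using a swept world offset.
; A sphere overlap calls Down on a hit target and destroys the bullet on any overlap, while a timer started at BeginPlay destroys it after a few seconds.
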(event OnComponentBeginOverlap(Sphere1)
  (params (OverlappedComponent :type Primitive%20Component%20Object%20Reference) (OtherActor :type Actor%20Object%20Reference) (OtherComp :type Primitive%20Component%20Object%20Reference) (OtherBodyIndex :type Integer) (bFromSweep :type Boolean) (SweepResult :type Hit%20Result%20Structure%20%28by%20ref%29))
  (Utilities|FlowControl|Sequence
    (:then_0
      (bind _astarget_bp (Utilities|Casting|CastToTarget_BP OtherActor))
      (Default|Down _astarget_bp))
    (:then_1
      (Actor|DestroyActor))))

(event Custom|destroy
  (Actor|DestroyActor))

(event EventTick
  (params (DeltaSeconds :type Float%20%28single-precision%29))
  (CallFunction|MoveForward (Variables|Default|Getspeed) DeltaSeconds))

(event EventBeginPlay
  (Utilities|Time|SetTimerbyEvent (delegate Custom|destroy) 4.0))

(fn ConstructionScript)

(fn MoveForward
  (params (Speed :type Float%20%28double-precision%29) (Timedelta :type Float%20%28double-precision%29))
  (Transformation|AddActorWorldOffset (* (* Speed Timedelta) (Math|Vector|GetForwardVector (Transformation|GetActorRotation))) true))